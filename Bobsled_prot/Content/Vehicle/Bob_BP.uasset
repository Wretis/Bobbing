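; Player-controlled bobsled Blueprint that drives the sled along the track with physics forces and lean-left/right steering.
; Each tick, a downward trace aligns it to the surface and adds capped forward force, reduced by yaw and boosted while both leans are held.
; Turning interpolates yaw within a clamped angle, recentring when neither or both are held.
; The camera widens FOV from velocity and uses either first-person look or a velocity-offset chase view.
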(event `InputAction|LeanLeft`
  (params (Key :type "Key Structure"))
  ;[1 1 1] Set currently held steering
  (:`Pressed`
    (set `self.LeaningLeft` true))
  (:`Released`
    (set `self.LeaningLeft` false)))

(event `InputAction|LeanRight`
  (params (Key :type "Key Structure"))
  ;[1 1 1] Set currently held steering
  (:`Pressed`
    (set `self.LeaningRight` true))
  (:`Released`
    (set `self.LeaningRight` false)))

(event `self.ReceiveTick`
  (params (DeltaSeconds :type "Float (single-precision)"))
  (bind _returnvalue (`self.K2_GetActorLocation`))
  (bind _bob (`self.Bob`))
  (bind _bob_cam1 (`self.Bob_Cam1`))
  (bind (_relativerotation_roll _relativerotation_pitch _relativerotation_yaw) (`KismetMathLibrary.BreakRotator` (`SceneComponent.RelativeRotation` (`self.Bob`))))
  (bind _returnvalue_2 (- (.x (* (`KismetMathLibrary.Normal` (`SceneComponent.GetForwardVector` _bob)) 1000.0)) (* (`KismetMathLibrary.SelectFloat` (* _relativerotation_yaw -1.0) _relativerotation_yaw (< _relativerotation_yaw 0.0)) 10.0)))
  (`|ExecutionSequence`
    (:`then_0`
      (if (and (`self.LeaningLeft`) (`self.LeaningRight`))
        (set `self.Holding` true)
        (else
          (set `self.Holding` false)))
      (bind (_outhit _returnvalue_3) (`KismetSystemLibrary.LineTraceSingle` :`Start` _returnvalue :`End` (+ _returnvalue (* (`self.GetActorUpVector`) -500.0)) :`TraceChannel` "TraceTypeQuery1" :`bTraceComplex` true :`DrawDebugType` "ForOneFrame"))
      (if _returnvalue_3
        (bind (_bblockinghit _binitialoverlap _time _distance _location _impactpoint _normal) (`GameplayStatics.BreakHitResult` _outhit))
        (`self.K2_SetActorRotation` (`KismetMathLibrary.MakeRotFromXZ` (`KismetMathLibrary.ProjectVectorOnToPlane` (`self.GetActorForwardVector`) _normal) _normal))
        (if _returnvalue_3
          (bind _returnvalue_4 (`PrimitiveComponent.GetPhysicsLinearVelocity` (`self.Bob`) "None"))
          (if (< (.x _returnvalue_4) (`self.MaxAcceleration`))
            (`PrimitiveComponent.AddForce` _bob (`KismetMathLibrary.MakeVector` (`KismetMathLibrary.SelectFloat` (+ _returnvalue_2 800.0) _returnvalue_2 (`self.Holding`)) (.y (* (`KismetMathLibrary.Normal` (`SceneComponent.GetForwardVector` _bob)) 1000.0)) (.z (* (`KismetMathLibrary.Normal` (`SceneComponent.GetForwardVector` _bob)) 1000.0))) "None" true)))))
    (:`then_1`
      (`self.Turning`)
      (bind _returnvalue_5 (`PrimitiveComponent.GetPhysicsLinearVelocity` (`self.Bob`) "None"))
      (`CameraComponent.SetFieldOfView` _bob_cam1 (+ (/ (.x _returnvalue_5) 1000000.0) (`CameraComponent.FieldOfView` _bob_cam1)))
      (if (`self.First-person?`)
        (`self.First-person camera`)
        (else
          (`self.Third-person camera`))))))

(event `self.ReceiveBeginPlay`
  (`self.EnableInput` null)
  (bind _returnvalue (`AddComponent|NODE_AddProjectileMovementComponent-1`))
  (set `self.ProjectileMovementReference` _returnvalue)
  (if (`self.First-person?`)
    (`SceneComponent.K2_AttachToComponent` (`self.Bob_Cam1`) (`self.Sledder2`) "headSocket" "KeepRelative" "KeepRelative" "KeepRelative" true)
    (else
      (`SceneComponent.K2_DetachFromComponent` (`self.Bob_Cam1`) "KeepRelative" "KeepRelative" "KeepRelative" true))))

(event `InputAxis|MoveRight`
  (params (AxisValue :type "Float (single-precision)"))
  (`PrimitiveComponent.AddTorqueInDegrees` (`self.Bob`) (0.0 0.0 0.0) "None" true)
  (if true
    _))

(fn `First-person camera`
  (bind _bob_cam1 (`self.Bob_Cam1`))
  (bind (_returnvalue_roll _returnvalue_pitch _returnvalue_yaw) (`KismetMathLibrary.BreakRotator` (`SceneComponent.K2_GetComponentRotation` _bob_cam1)))
  (`SceneComponent.K2_SetWorldRotation` _bob_cam1 (`KismetMathLibrary.MakeRotator` 0.0 (+ (* (`self.GetInputAxisValue`) -1.0) _returnvalue_pitch) (+ (`self.GetInputAxisValue`) _returnvalue_yaw)) false false))

(fn `Third-person camera`
  (bind _bob (`self.Bob`))
  (bind _bob_cam1 (`self.Bob_Cam1`))
  (bind _returnvalue_x (`KismetMathLibrary.BreakVector` (`SceneComponent.GetComponentVelocity` _bob)))
  (bind _returnvalue (`SceneComponent.K2_GetComponentLocation` _bob))
  (bind _returnvalue_2 (/ _returnvalue_x 80.0))
  (bind (_returnvalue_roll _returnvalue_pitch _returnvalue_yaw) (`KismetMathLibrary.BreakRotator` (`KismetMathLibrary.FindLookAtRotation` (`SceneComponent.K2_GetComponentLocation` _bob_cam1) _returnvalue)))
  (`SceneComponent.K2_SetWorldLocation` _bob_cam1 (`KismetMathLibrary.MakeVector` (- (.x _returnvalue) (- 200.0 _returnvalue_2)) (.y _returnvalue) (+ (.z _returnvalue) 300.0 (/ _returnvalue_2 10.0))) false false)
  (`SceneComponent.K2_SetWorldRotation` _bob_cam1 (`KismetMathLibrary.MakeRotator` _returnvalue_roll (+ _returnvalue_pitch 15.0) _returnvalue_yaw) false false))

(fn `Turning`
  (bind _turnratio (`self.TurnRatio`))
  (bind (_returnvalue_roll _returnvalue_pitch _returnvalue_yaw) (`KismetMathLibrary.BreakRotator` (`self.K2_GetActorRotation` self)))
  (bind _returnvalue (`KismetMathLibrary.Conv_BoolToDouble` (`self.LeaningRight`)))
  (bind _returnvalue_2 (`KismetMathLibrary.Conv_BoolToDouble` (`self.LeaningLeft`)))
  (`self.K2_SetActorRotation` self (`KismetMathLibrary.MakeRotator` _returnvalue_roll _returnvalue_pitch (`KismetMathLibrary.FInterpTo` _returnvalue_yaw (`KismetMathLibrary.SelectFloat` 0.0 (`KismetMathLibrary.FClamp` (+ _returnvalue_yaw (+ (* (* _returnvalue_2 -1.0) _turnratio) (* _returnvalue _turnratio))) (* (`self.MaxTurnAngle`) -1.0) (`self.MaxTurnAngle`)) (or (== (+ _returnvalue_2 _returnvalue) 0.0) (`self.Holding`))) (`GameplayStatics.GetWorldDeltaSeconds`) 5.0)) false))

(fn `UserConstructionScript`)