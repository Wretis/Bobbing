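; Actor that poses a poseable mesh character's legs and spine, apparently as a rider attached to a parent actor.
; The construction script offsets thigh and calf bone rotations in world space to set a fixed leg pose.
; Each tick eases spine_01 toward its BeginPlay rotation plus the parent's yaw.
; A pitched lean target exists but is never selected, and the stored LeaningLeft flag is unused.
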(event `GetBobLeaningLeft`
  (params (`CurrentlyLeaning?` :type Boolean))
  (set `self.LeaningLeft` `CurrentlyLeaning?`))

(event `self.ReceiveBeginPlay`
  (bind _returnvalue (`PoseableMeshComponent.GetBoneRotationByName` (`self.PoseableMesh`) "spine_01" "WorldSpace"))
  (set `self.SpineRotation` _returnvalue))

(event `self.ReceiveTick`
  (params (DeltaSeconds :type "Float (single-precision)"))
  (bind _poseablemesh (`self.PoseableMesh`))
  (bind (_returnvalue_roll _returnvalue_pitch _returnvalue_yaw) (`KismetMathLibrary.BreakRotator` (`self.K2_GetActorRotation` (`self.GetParentActor`))))
  (bind _returnvalue (`KismetMathLibrary.MakeRotator` (.roll (`self.SpineRotation`)) (.pitch (`self.SpineRotation`)) (+ (.yaw (`self.SpineRotation`)) _returnvalue_yaw)))
  (bind _returnvalue_2 (`PoseableMeshComponent.GetBoneRotationByName` _poseablemesh "spine_01" "WorldSpace"))
  (`PoseableMeshComponent.SetBoneRotationByName` _poseablemesh "spine_01" (`KismetMathLibrary.RInterpTo` _returnvalue_2 (`KismetMathLibrary.SelectRotator` (`KismetMathLibrary.MakeRotator` (.roll _returnvalue) (+ (.pitch _returnvalue) 90.0) (.yaw _returnvalue)) _returnvalue) (`GameplayStatics.GetWorldDeltaSeconds`) 5.0) "WorldSpace"))

(fn `UserConstructionScript`
  (bind _poseablemesh (`self.PoseableMesh`))
  (bind _returnvalue (`PoseableMeshComponent.GetBoneRotationByName` _poseablemesh "thigh_r" "WorldSpace"))
  (`PoseableMeshComponent.SetBoneRotationByName` _poseablemesh "thigh_r" (`KismetMathLibrary.MakeRotator` (+ (.roll _returnvalue) -90.0) (+ (.pitch _returnvalue) -90.0) (+ (.yaw _returnvalue) 90.0)) "WorldSpace")
  (bind _returnvalue_2 (`PoseableMeshComponent.GetBoneRotationByName` _poseablemesh "thigh_l" "WorldSpace"))
  (`PoseableMeshComponent.SetBoneRotationByName` _poseablemesh "thigh_l" (`KismetMathLibrary.MakeRotator` (+ (.roll _returnvalue_2) 90.0) (+ (.pitch _returnvalue_2) -90.0) (+ (.yaw _returnvalue_2) 90.0)) "WorldSpace")
  (bind _returnvalue_3 (`PoseableMeshComponent.GetBoneRotationByName` _poseablemesh "calf_r" "WorldSpace"))
  (`PoseableMeshComponent.SetBoneRotationByName` _poseablemesh "calf_r" (`KismetMathLibrary.MakeRotator` (+ (.roll _returnvalue_3) -90.0) (+ (.pitch _returnvalue_3) -90.0) (+ (.yaw _returnvalue_3) 90.0)) "WorldSpace")
  (bind _returnvalue_4 (`PoseableMeshComponent.GetBoneRotationByName` _poseablemesh "calf_l" "WorldSpace"))
  (`PoseableMeshComponent.SetBoneRotationByName` _poseablemesh "calf_l" (`KismetMathLibrary.MakeRotator` (+ (.roll _returnvalue_4) 90.0) (+ (.pitch _returnvalue_4) 90.0) (+ (.yaw _returnvalue_4) 90.0)) "WorldSpace"))